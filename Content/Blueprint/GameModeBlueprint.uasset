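; Game mode Blueprint that can fill the level with a grid of actors, apparently spaceships, when play begins.
; If the SpawnSpaceshipsText flag is set, BeginPlay runs nested row and column loops that spawn the Template class on the XY plane at SpaceBetween intervals from the world origin.
; Both loops include their end index, so the grid has one more row and column than NumRow and NumCol.
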(event `self.ReceiveBeginPlay`
  (bind _spacebetween (`self.SpaceBetween`))
  (if (`self.Spawn_Spaceships_Text`)
    (for _index (range (+ (`self.NumRow`) 1))
      (for _index_2 (range (+ (`self.NumCol`) 1))
        (`|SpawnActorFromClass` (`self.Template`) (`KismetMathLibrary.MakeTransform` (`KismetMathLibrary.MakeVector` (* _index_2 _spacebetween) (* _index _spacebetween))) "Undefined" "OverrideRootScale")))))

(fn `UserConstructionScript`)